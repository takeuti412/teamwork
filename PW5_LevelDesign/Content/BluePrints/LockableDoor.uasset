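; A hinged door that opens when something overlaps its Box trigger and, if locked, requires the player to carry its KeyItem.
; For a locked door, the player controller's inventory is searched for the key; a match unlocks and opens it with debug prints.
; A timeline drives DoorRoot yaw, reversing when the player exits with AutoClose set.
; An elapsed-time counter, reset on closing, briefly blocks retriggering.
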(event OnComponentBeginOverlap(Box)
  (params (OverlappedComponent :type Primitive%20Component%20Object%20Reference) (OtherActor :type Actor%20Object%20Reference) (OtherComp :type Primitive%20Component%20Object%20Reference) (OtherBodyIndex :type Integer) (bFromSweep :type Boolean) (SweepResult :type Hit%20Result%20Structure%20%28by%20ref%29))
  (if (>= (Variables|Default|GetElapsedTime) 0.5)
    (Variables|Default|SetOverlapping true)
    (if (Variables|Default|GetClosed)
      (if (Variables|Default|GetLocked)
        (if (== OtherActor (Game|Player|GetPlayerPawn 0))
          ;[1 1 1] Playerの持ってるアイテムから変数 Key Item と一致する物を探す
          (bind _asplayer_character_controller (Utilities|Casting|CastToPlayerCharacterController (Game|GetPlayerController 0)))
          (for _array_element (Variables|/Game/BluePrints/PlayerCharacterController.PlayerCharacterController_C|GetInv _asplayer_character_controller)
            ;;[1 1 1] KeyItemがNoneでも開いちゃう
            (if (== _array_element (Variables|Default|GetKeyItem))
              (CallFunction|Unlock))))
        (else
          (CallFunction|OpenDoor))))))

(event OnComponentEndOverlap(Box)
  (params (OverlappedComponent :type Primitive%20Component%20Object%20Reference) (OtherActor :type Actor%20Object%20Reference) (OtherComp :type Primitive%20Component%20Object%20Reference) (OtherBodyIndex :type Integer))
  (Variables|Default|SetOverlapping false)
  (if (not (Variables|Default|GetClosed))
    (if (Variables|Default|GetAutoClose)
      (if (== OtherActor (Game|Player|GetPlayerPawn 0))
        (CallFunction|CloseDoor)
        (Variables|Default|SetElapsedTime 0.0)))))

(event Custom|OpenDoor
  (Variables|Default|SetClosed false)
  (bind _newtrack_0 (Timeline|DoorOpen Play)
    (:Update
      (Transformation|SetRelativeRotation (Variables|Default|GetDoorRoot) (Math|Rotator|MakeRotator 0.0 0.0 _newtrack_0) false false))))

(event Custom|Unlock
  (Variables|Default|SetLocked false)
  (CallFunction|OpenDoor)
  (Development|PrintString (Utilities|String|Append "The key, \"" (Utilities|GetDisplayName (Variables|Default|GetKeyItem)) "\" is used"))
  (Development|PrintString (Utilities|String|Append "The door, \"" (Utilities|String|ToString(Object) self) "\" is unlocked")))

(event Custom|CloseDoor
  (Variables|Default|SetClosed true)
  (bind _newtrack_0 (Timeline|DoorOpen Reverse)
    (:Update
      (Transformation|SetRelativeRotation (Variables|Default|GetDoorRoot) (Math|Rotator|MakeRotator 0.0 0.0 _newtrack_0) false false))))

(event EventTick
  (params (DeltaSeconds :type Float%20%28single-precision%29))
  (Variables|Default|SetDeltaTime DeltaSeconds)
  (Variables|Default|SetElapsedTime (+ (Variables|Default|GetElapsedTime) (Variables|Default|GetDeltaTime))))

(fn ConstructionScript)